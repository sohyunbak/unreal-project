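; Actor Blueprint that polls a VisionRelay HTTP API for the people count reported for a given camera ID.
; A looping timer started on BeginPlay sends a GET request each tick, skipped while StatusSwaper is idle.
; Successful responses are parsed as JSON and the personCount field is stored in CurrentPeopleCount; failed requests only print a message.
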(event Custom|GetData
  (if (not (Variables|/Game/CMS/Blueprints/BP_StatusSwaper.BP_StatusSwaper_C|GetIsIdle (Variables|Default|GetStatusSwaper)))
    (bind _result_body (|HttpRequest (Utilities|String|Append (Variables|Default|GetHostURL) (Variables|Default|GetVisionRelayDateAPIURL) (Variables|Default|GetCameraID)) "Get")
      (:then
        (Development|PrintString "VisionRelay: Requesting"))
      (:On%20Success
        (bind _outjsonobject (Class|JsonBlueprintFunctionLibrary|FromString _result_body))
        (bind (_outvalue _returnvalue) (|GetJsonField _outjsonobject "personCount"))
        (if _returnvalue
          (Variables|Default|SetCurrentPeopleCount (Math|Conversions|ToInteger(Byte) _outvalue))))
      (:On%20Error
        (Development|PrintString "VisionRelay: Request Failed")))))

(event EventBeginPlay
  (Utilities|Time|SetTimerbyEvent (delegate Custom|GetData) (Variables|Default|GetTimerTick) true))

(event Collision|EventActorBeginOverlap
  (params (OtherActor :type Actor%20Object%20Reference)))

(event EventTick
  (params (DeltaSeconds :type Float%20%28single-precision%29)))

(fn ConstructionScript)