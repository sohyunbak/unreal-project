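; BP_StatusBroadCaster reports the idle or active state of a StatusSwaper to external systems.
; A looping timer sends the matching idle or active packet over UDP on the PlaymonSender channel.
; On each StatusSwaper state change it resends that packet immediately and calls the VisionRelay pause or start HTTP GET endpoint to match, printing successful responses.
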(event Custom|SendStateMessage
  (Class|SimpleUDPSubsystem|SendUDPMessage "PlaymonSender" (Class|SimpleByteConversionBPLibrary|StringtoBytes (Utilities|String|MakeLiteralString (Utilities|String|SelectString (Variables|Default|GetIdlePacketData) (Variables|Default|GetActivePacketData) (Variables|/Game/CMS/Blueprints/BP_StatusSwaper.BP_StatusSwaper_C|GetIsIdle (Variables|Default|GetStatusSwaper)))))))

(event Custom|OnStateChange
  (bind _statusswaper (Variables|Default|GetStatusSwaper))
  (bind _hosturl (Variables|Default|GetHostURL))
  (bind _isidle (Variables|/Game/CMS/Blueprints/BP_StatusSwaper.BP_StatusSwaper_C|GetIsIdle _statusswaper))
  (Class|SimpleUDPSubsystem|SendUDPMessage "PlaymonSender" (Class|SimpleByteConversionBPLibrary|StringtoBytes (Utilities|String|MakeLiteralString (Utilities|String|SelectString (Variables|Default|GetIdlePacketData) (Variables|Default|GetActivePacketData) _isidle))))
  (if _isidle
    (bind _result_body (|HttpRequest (Utilities|String|Append _hosturl (Variables|Default|GetVisionRelayPauseAPIURL)) "Get")
      (:On%20Success
        (Development|PrintString _result_body)))
    (else
      (bind _result_body_2 (|HttpRequest (Utilities|String|Append _hosturl (Variables|Default|GetVisionRelayStartAPIURL)) "Get")
        (:On%20Success
          (Development|PrintString _result_body_2))))))

(event EventBeginPlay
  (Utilities|Time|SetTimerbyEvent (delegate Custom|SendStateMessage) (Variables|Default|GetTimerTick) true)
  (EventDispatchers|BindEventtoOnStateChange (Variables|Default|GetStatusSwaper) (delegate Custom|OnStateChange)))

(event Collision|EventActorBeginOverlap
  (params (OtherActor :type Actor%20Object%20Reference)))

(event EventTick
  (params (DeltaSeconds :type Float%20%28single-precision%29)))

(fn ConstructionScript)