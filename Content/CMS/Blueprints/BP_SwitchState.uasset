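; Blueprint function that switches the game between a low-cost idle state and the active state.
; Idle throttles frame rate and screen percentage, covers the viewport with a returned BlackScreen widget, and nearly freezes time dilation.
; It also hides and stops ticking every actor not tagged "Comm".
; Active removes the passed-in widget, resets those settings, and re-enables ticking and visibility on all untagged actors, regardless of their earlier state.
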(fn SwitchState
  (params (SwapToIdle :type Boolean) (BlackScreenRef :type Black%20Screen%20Object%20Reference))
  (if SwapToIdle
    (Development|PrintString 0 "ToIdle")
    (Development|ExecuteConsoleCommand 0 "t.MaxFPS 5" 0)
    (Development|ExecuteConsoleCommand 0 "r.ScreenPercentage 10" 0)
    (bind _returnvalue (UserInterface|CreateWidget 0 "/Game/CMS/UIs/BlackScreen.BlackScreen_C" (Game|GetPlayerController 0)))
    (UserInterface|Viewport|AddtoViewport _returnvalue 999)
    (bind _outactors (Actor|GetAllActorsOfClass 0 "/Script/Engine.Actor"))
    (for _array_element _outactors
      (if (not (Actor|ActorHasTag _array_element "Comm"))
        (Actor|Tick|SetActorTickEnabled _array_element)
        (Rendering|SetActorHiddenInGame _array_element true)))
    (Utilities|Time|SetGlobalTimeDilation 0 0.01)
    (return _returnvalue)
    (else
      (Development|PrintString 0 "ToActive")
      (Widget|RemovefromParent BlackScreenRef)
      (Development|ExecuteConsoleCommand 0 "t.MaxFPS 0" 0)
      (Development|ExecuteConsoleCommand 0 "r.ScreenPercentage 100" 0)
      (bind _outactors_2 (Actor|GetAllActorsOfClass 0 "/Script/Engine.Actor"))
      (for _array_element_2 _outactors_2
        (if (not (Actor|ActorHasTag _array_element_2 "Comm"))
          (Actor|Tick|SetActorTickEnabled _array_element_2 true)
          (Rendering|SetActorHiddenInGame _array_element_2 false)))
      (Utilities|Time|SetGlobalTimeDilation 0 1.0))))