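; Actor that switches the game between idle and active states from UDP messages, starting idle.
; Idle packets start a delayed transition that an active packet cancels; active packets wake immediately.
; SwitchState handles each swap with a black-screen reference, then OnStateChange is broadcast; EndPlay resets frame-rate and screen-percentage console settings.
; Debug keys toggle the state and adjust the idle delay.
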(event Custom|커스텀이벤트
  (params (SenderIP :type String) (SenderPort :type Integer%20%28by%20ref%29) (Message :type Array%20of%20Bytes))
  (bind _value (Class|SimpleByteConversionBPLibrary|BytestoString Message))
  (bind _activepacketdata (Variables|Default|GetActivePacketData))
  (bind _isidle (Variables|Default|GetIsIdle))
  (bind _returnvalue (Utilities|Enum|Equal(Enum) _value _activepacketdata))
  (bind _returnvalue_2 (not _isidle))
  (Development|PrintString (Utilities|String|Append SenderIP _value))
  (if (and (Utilities|Enum|Equal(Enum) _value (Variables|Default|GetIdlePacketData)) _returnvalue_2)
    (if (not (Utilities|Time|IsTimerActivebyHandle (Variables|Default|GetIdleHandler)))
      (bind _returnvalue_3 (Utilities|Time|SetTimerbyEvent (delegate Custom|ToIdleMode) (Variables|Default|GetIdleAwaitTime)))
      (Variables|Default|SetIdleHandler _returnvalue_3)
      (Development|PrintText "Preparing Idle State"))
    (elif (and _returnvalue _isidle)
      (CallFunction|ToActiveMode)
      (elif (Math|Boolean|ANDBoolean _returnvalue _returnvalue_2 (Utilities|Time|IsTimerActivebyHandle (Variables|Default|GetIdleHandler)))
        (Utilities|Time|ClearandInvalidateTimerbyHandle (Variables|Default|GetIdleHandler))
        (Development|PrintString "Transition Cancelled")))))

(event Custom|ToIdleMode
  (Utilities|FlowControl|Delay 0.05)
  (if (and (not (Utilities|Time|IsTimerActivebyHandle (Variables|Default|GetIdleHandler))) (not (Variables|Default|GetIsIdle)))
    (bind _outputblackscreen (CallFunction|SwitchState true))
    (Variables|Default|SetBlackScreenRef _outputblackscreen)
    (Variables|Default|SetIsIdle true)
    (Default|CallOnStateChange)))

(event Custom|ToActiveMode
  (if (Variables|Default|GetIsIdle)
    (CallFunction|SwitchState false (Variables|Default|GetBlackScreenRef))
    (Variables|Default|SetIsIdle false)
    (Default|CallOnStateChange)
    (elif (Math|Boolean|ANDBoolean (Utilities|Enum|Equal(Enum) (Class|SimpleByteConversionBPLibrary|BytestoString (stale Custom|커스텀이벤트 Message)) (Variables|Default|GetActivePacketData)) (not (Variables|Default|GetIsIdle)) (Utilities|Time|IsTimerActivebyHandle (Variables|Default|GetIdleHandler)))
      (Utilities|Time|ClearandInvalidateTimerbyHandle (Variables|Default|GetIdleHandler))
      (Development|PrintString "Transition Cancelled"))))

(event EventBeginPlay
  (Variables|/Script/Engine.Actor|SetTags (Game|GetPlayerController 0) (Variables|Default|GetTags_0))
  (Development|ExecuteConsoleCommand "r.FullScreenMode 1" 0)
  (bind _outputblackscreen (CallFunction|SwitchState true))
  (Variables|Default|SetBlackScreenRef _outputblackscreen)
  (Variables|Default|SetIsIdle true)
  (Default|CallOnStateChange)
  (Class|SimpleUDPSubsystem|BindUDPMessageHandler "PlaymonReceiver" (delegate Custom|커스텀이벤트)))

(event Collision|EventActorBeginOverlap
  (params (OtherActor :type Actor%20Object%20Reference)))

(event EventTick
  (params (DeltaSeconds :type Float%20%28single-precision%29)))

(event EventEndPlay
  (params (EndPlayReason :type EEndPlayReason%20Enum :default "Destroyed"))
  (Development|ExecuteConsoleCommand "t.MaxFPS 0" 0)
  (Development|ExecuteConsoleCommand "r.ScreenPercentage 100" 0))

(event Input|KeyboardEvents|Up
  (params (Key :type Key%20Structure :default "None"))
  (:Pressed
    (Variables|Default|SetIdleAwaitTime (Math|Float|Clamp(Float) (+ (Variables|Default|GetIdleAwaitTime) 0.1) 0.01 1e+01))
    (Development|PrintString (Utilities|String|Append "Variable updated to" (Utilities|String|ToString(Float) (Variables|Default|GetIdleAwaitTime))))))

(event Input|KeyboardEvents|Down
  (params (Key :type Key%20Structure :default "None"))
  (:Pressed
    (Variables|Default|SetIdleAwaitTime (Math|Float|Clamp(Float) (- (Variables|Default|GetIdleAwaitTime) 0.1) 0.01 1e+01))
    (Development|PrintString (Utilities|String|Append "Variable updated to" (Utilities|String|ToString(Float) (Variables|Default|GetIdleAwaitTime))))))

(event Input|KeyboardEvents|1
  (params (Key :type Key%20Structure :default "None"))
  (:Pressed
    (if (Variables|Default|GetIsIdle)
      (CallFunction|ToActiveMode)
      (else
        (CallFunction|ToIdleMode)))))

(fn ConstructionScript)