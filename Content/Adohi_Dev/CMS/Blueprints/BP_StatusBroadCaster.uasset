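; Status broadcaster actor that relays state to an external receiver over UDP and HTTP.
; On BeginPlay it starts a looping timer that sends a packet on the PlaymonSender UDP channel, and binds to StatusSwaper's state change.
; A state change resends the packet and calls the vision relay pause API when idle, or start otherwise.
; Both sends always select the active packet, as PickA is fixed false.
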(event Custom|SendStateMessage
  (Class|SimpleUDPSubsystem|SendUDPMessage "PlaymonSender" (Class|SimpleByteConversionBPLibrary|StringtoBytes (Utilities|String|MakeLiteralString (Utilities|String|SelectString (Variables|Default|GetIdlePacketData) (Variables|Default|GetActivePacketData) false)))))

(event Custom|OnStateChange
  (bind _hosturl (Variables|Default|GetHostURL))
  (Class|SimpleUDPSubsystem|SendUDPMessage "PlaymonSender" (Class|SimpleByteConversionBPLibrary|StringtoBytes (Utilities|String|MakeLiteralString (Utilities|String|SelectString (Variables|Default|GetIdlePacketData) (Variables|Default|GetActivePacketData) false))))
  (if (Variables|/Game/Adohi_Dev/CMS/Blueprints/BP_StatusSwaper.BP_StatusSwaper_C|GetIsIdle (Variables|Default|GetStatusSwaper))
    (bind _result_body (|HttpRequest (Utilities|String|Append _hosturl (Variables|Default|GetVisionRelayPauseAPIURL)) "Get")
      (:On%20Success
        (Development|PrintString _result_body true false)))
    (else
      (bind _result_body_2 (|HttpRequest (Utilities|String|Append _hosturl (Variables|Default|GetVisionRelayStartAPIURL)) "Get")
        (:On%20Success
          (Development|PrintString _result_body_2 true false))))))

(event EventBeginPlay
  (Utilities|Time|SetTimerbyEvent (delegate Custom|SendStateMessage) (Variables|Default|GetTimerTick) true)
  (EventDispatchers|BindEventtoOnStateChange (Variables|Default|GetStatusSwaper) (delegate Custom|OnStateChange)))

(event Collision|EventActorBeginOverlap
  (params (OtherActor :type Actor%20Object%20Reference)))

(event EventTick
  (params (DeltaSeconds :type Float%20%28single-precision%29)))

(fn ConstructionScript)