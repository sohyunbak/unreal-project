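; Actor that polls a Vision Relay HTTP API for the person count seen by a given camera ID.
; A self-rearming timer sends a GET request unless StatusSwaper is idle, then stores the JSON personCount in CurrentPeopleCount.
; Failed requests double the polling interval up to a maximum, and a successful response resets it to the default.
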(event Custom|GetData
  (if (Variables|/Game/Adohi_Dev/CMS/Blueprints/BP_StatusSwaper.BP_StatusSwaper_C|GetIsIdle (Variables|Default|GetStatusSwaper))
    (Utilities|Time|SetTimerbyEvent (delegate Custom|GetData) (Variables|Default|GetCurrentTimerTick) :!label _label)
    (else
      (Development|PrintString "Log_Request" true false)
      (bind _result_body (|HttpRequest (Utilities|String|Append (Variables|Default|GetHostURL) (Variables|Default|GetVisionRelayDateAPIURL) (Variables|Default|GetCameraID)) "Get")
        (:then
          (Development|PrintString "VisionRelay: Requesting" true false))
        (:On%20Success
          (bind _outjsonobject (Class|JsonBlueprintFunctionLibrary|FromString _result_body))
          (bind (_outvalue _returnvalue) (|GetJsonField _outjsonobject "personCount"))
          (if _returnvalue
            (Variables|Default|SetCurrentPeopleCount (Math|Conversions|ToInteger(Byte) _outvalue)))
          (Variables|Default|SetCurrentTimerTick (Variables|Default|GetDefaultTimerTick))
          (goto _label))
        (:On%20Error
          (Development|PrintString "VisionRelay: Request Failed" true false)
          (Variables|Default|SetCurrentTimerTick (Math|Float|Clamp(Float) (* (Variables|Default|GetCurrentTimerTick) 2.0) (Variables|Default|GetDefaultTimerTick) (Variables|Default|GetMaxTimerTick)))
          (goto _label))))))

(event EventBeginPlay
  (Variables|Default|SetCurrentTimerTick (Variables|Default|GetDefaultTimerTick))
  (Utilities|Time|SetTimerbyEvent (delegate Custom|GetData) (Variables|Default|GetCurrentTimerTick)))

(event Collision|EventActorBeginOverlap
  (params (OtherActor :type Actor%20Object%20Reference)))

(event EventTick
  (params (DeltaSeconds :type Float%20%28single-precision%29)))

(fn ConstructionScript)