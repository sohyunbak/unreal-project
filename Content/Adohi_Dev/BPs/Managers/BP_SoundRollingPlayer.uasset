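; BP_SoundRollingPlayer is a manager actor that plays 2D sounds from an array in round-robin order.
; On BeginPlay it registers itself as SoundRoller on BP_GameInstance.
; PlaySound spawns the sound at CurrentIndex and keeps its audio component.
; StopSound stops that component and advances the index, wrapping around, so the next play uses the following sound.
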(event EventBeginPlay
  (bind _asbp_game_instance (Utilities|Casting|CastToBP_GameInstance (Game|GetGameInstance)))
  (Variables|/Game/Adohi_Dev/CMS/Blueprints/BP_GameInstance.BP_GameInstance_C|SetSoundRoller _asbp_game_instance self))

(event Collision|EventActorBeginOverlap
  (params (OtherActor :type Actor%20Object%20Reference)))

(event EventTick
  (params (DeltaSeconds :type Float%20%28single-precision%29)))

(fn ConstructionScript)

(fn PlaySound
  (bind _returnvalue (Audio|SpawnSound2D (Utilities|Array|Get(acopy) (Variables|Default|GetSounds) (Variables|Default|GetCurrentIndex)) 1.0 1.0 0.0 0))
  (Variables|Default|SetSoundComponent _returnvalue))

(fn StopSound
  (Audio|Components|Audio|Stop (Variables|Default|GetSoundComponent))
  (Variables|Default|SetCurrentIndex (Math|Integer|%(Integer) (+ (Variables|Default|GetCurrentIndex) 1) (Utilities|Array|Length (Variables|Default|GetSounds)))))