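; A child butterfly actor that follows a spline path and shows or hides itself based on a game-wide butterfly control value.
; On BeginPlay it caches the game instance and assigns its path reference as the spline follower component's parent spline.
; Every tick it hides itself unless the MAController's butterfly control value exceeds its spawn threshold by a small margin.
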(event EventBeginPlay
  (|CallParentFunction)
  (bind _asbp_game_instance (Utilities|Casting|CastToBP_GameInstance (Game|GetGameInstance)))
  (Variables|/Game/Adohi_Dev/BPs/MAAssets/Butterflies/BP_SplineFollower.BP_SplineFollower_C|SetSplineParent (Variables|Default|GetBP_SplineFollower) (Variables|Default|GetPathRef)))

(event Collision|EventActorBeginOverlap
  (params (OtherActor :type Actor%20Object%20Reference))
  (|CallParentFunction OtherActor) ; This node is disabled and will not be called.\nDrag off pins to build functionality.
)

(event EventTick
  (params (DeltaSeconds :type Float%20%28single-precision%29))
  (|CallParentFunction DeltaSeconds)
  (Rendering|SetActorHiddenInGame (<= (Variables|/Game/Adohi_Dev/BPs/MAControls/BP_MAController.BP_MAController_C|GetButterflyControlValue (Variables|/Game/Adohi_Dev/CMS/Blueprints/BP_GameInstance.BP_GameInstance_C|GetMAController (stale EventBeginPlay _asbp_game_instance))) (+ (Variables|Default|GetSpawnThreshold) 0.01))))

(fn ConstructionScript
  (|CallParentFunction))