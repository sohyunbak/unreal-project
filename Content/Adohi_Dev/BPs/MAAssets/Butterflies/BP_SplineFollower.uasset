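; Component that flies its owning butterfly actor around a looping spline while visibility is desired, and sends it back to hide when not.
; SetupSpline and SetDesiredVisibleState feed a Tick state machine: rejoin, follow, return to spline start, hidden.
; Rejoining steers forward toward a look-ahead point from the closest spline position, switching turn rate when near.
; Sine-modulated speed varies the flight, and quaternion slerp smooths turning.
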(event EventBeginPlay
  (Utilities|FlowControl|Sequence
    (:then_0
      (Rendering|SetActorHiddenInGame (Components|GetOwner) true :!label _label)
      (Variables|ButterflyState|SetButterflyState 3)
      (Variables|Default|SetCurrentDistance 0.0))
    (:then_1
      (if (not (Variables|ButterflyState|GetDesiredVisible))
        (goto _label)))))

(event EventTick
  (params (DeltaSeconds :type Float%20%28single-precision%29))
  (bind _returnvalue (Components|GetOwner))
  (bind _returnvalue_2 (Utilities|Time|GetGameTimeinSeconds))
  (bind _speedoscillationamplitude (Variables|ButterflyStyle|GetSpeedOscillationAmplitude))
  (bind _turninterpspeed (Variables|ButterflyState|GetTurnInterpSpeed))
  (bind _speedoscillationfrequency (Variables|ButterflyStyle|GetSpeedOscillationFrequency))
  (bind _arrivaltolerance (Variables|ButterflyState|GetArrivalTolerance))
  (bind _nearturninterpspeed (Variables|ButterflyState|GetNearTurnInterpSpeed))
  (bind _nearturndistance (Variables|ButterflyState|GetNearTurnDistance))
  (bind _splinecomp (Variables|Default|GetSplineComp))
  (bind _rejoinlookaheaddistance (Variables|ButterflyState|GetRejoinLookAheadDistance))
  (bind _desiredvisible (Variables|ButterflyState|GetDesiredVisible))
  (bind _speed (Variables|Default|GetSpeed))
  (bind _returnvalue_3 (Spline|GetSplineLength _splinecomp))
  (bind _returnvalue_4 (Transformation|GetActorLocation _returnvalue))
  (bind _returnvalue_5 (Spline|GetLocationatDistanceAlongSpline _splinecomp 0.0 "World"))
  (bind _returnvalue_6 (Transformation|GetActorLocation _returnvalue))
  (bind _returnvalue_7 (Transformation|GetActorRotation _returnvalue))
  (bind _returnvalue_8 (* _returnvalue_2 _speedoscillationfrequency))
  (bind _returnvalue_9 (Class|SplineComponent|FindInputKeyClosesttoWorldLocation _splinecomp _returnvalue_6))
  (bind _returnvalue_10 (Math|Conversions|ToQuaternion(Rotator) _returnvalue_7))
  (bind _returnvalue_11 (Math|Trig|Sin(Radians) _returnvalue_8))
  (bind _returnvalue_12 (Class|SplineComponent|GetDistanceAlongSplineatSplineInputKey _splinecomp _returnvalue_9))
  (bind _returnvalue_13 (* _returnvalue_11 _speedoscillationamplitude))
  (bind _returnvalue_14 (+ _returnvalue_12 _rejoinlookaheaddistance))
  (bind _returnvalue_15 (+ _returnvalue_13 1.0))
  (bind _returnvalue_16 (>= _returnvalue_14 _returnvalue_3))
  (bind _returnvalue_17 (* _speed _returnvalue_15))
  (bind _returnvalue_18 (* _returnvalue_17 DeltaSeconds))
  (bind _returnvalue_19 (Math|Interpolation|VInterptoConstant _returnvalue_4 _returnvalue_5 DeltaSeconds _returnvalue_17))
  (bind _returnvalue_20 (Math|Float|SelectFloat 0.0 _returnvalue_14 _returnvalue_16))
  (bind _returnvalue_21 (Spline|GetLocationatDistanceAlongSpline _splinecomp _returnvalue_20 "World"))
  (bind _returnvalue_22 (Math|Rotator|FindLookatRotation _returnvalue_6 _returnvalue_21))
  (bind _returnvalue_23 (- _returnvalue_21 _returnvalue_6))
  (bind _returnvalue_24 (Math|Vector|VectorLength _returnvalue_23))
  (bind _returnvalue_25 (Math|Conversions|ToQuaternion(Rotator) _returnvalue_22))
  (bind _returnvalue_26 (<= _returnvalue_24 _nearturndistance))
  (bind _returnvalue_27 (Math|Float|SelectFloat _nearturninterpspeed _turninterpspeed _returnvalue_26))
  (bind _returnvalue_28 (* DeltaSeconds _returnvalue_27))
  (bind _returnvalue_29 (Class|KismetMathLibrary|QuatSlerp _returnvalue_10 _returnvalue_25 _returnvalue_28))
  (bind _returnvalue_30 (Class|KismetMathLibrary|QuatRotator _returnvalue_29))
  (if _desiredvisible
    (if (Utilities|IsValid _splinecomp) :!label _label
      (if (== (Variables|ButterflyState|GetButterflyState) 1)
        (if _desiredvisible
          (Transformation|SetActorLocationAndRotation _returnvalue (Spline|GetLocationatDistanceAlongSpline _splinecomp (Math|Float|SelectFloat 0.0 (+ (Variables|Default|GetCurrentDistance) _returnvalue_18) (>= (+ (Variables|Default|GetCurrentDistance) _returnvalue_18) _returnvalue_3)) "World") (Class|KismetMathLibrary|QuatRotator (Class|KismetMathLibrary|QuatSlerp (Math|Conversions|ToQuaternion(Rotator) (Transformation|GetActorRotation _returnvalue)) (Math|Conversions|ToQuaternion(Rotator) (Spline|GetRotationatDistanceAlongSpline _splinecomp (Math|Float|SelectFloat 0.0 (+ (Variables|Default|GetCurrentDistance) _returnvalue_18) (>= (+ (Variables|Default|GetCurrentDistance) _returnvalue_18) _returnvalue_3)) "World")) (* DeltaSeconds _turninterpspeed))))
          (Variables|Default|SetCurrentDistance (Math|Float|SelectFloat 0.0 (+ (Variables|Default|GetCurrentDistance) _returnvalue_18) (>= (+ (Variables|Default|GetCurrentDistance) _returnvalue_18) _returnvalue_3)))
          (else
            (if (<= (Math|Vector|VectorLength (- _returnvalue_5 _returnvalue_19)) _arrivaltolerance) :!label _label_2
              (Rendering|SetActorHiddenInGame _returnvalue true :!label _label_3)
              (Variables|ButterflyState|SetButterflyState 3)
              (Variables|Default|SetCurrentDistance 0.0)
              (else
                (Variables|ButterflyState|SetButterflyState 2)))))
        (elif (== (Variables|ButterflyState|GetButterflyState) 2)
          (if _desiredvisible
            (Rendering|SetActorHiddenInGame _returnvalue false)
            (Variables|ButterflyState|SetButterflyState 0)
            (else
              (Transformation|SetActorLocationAndRotation _returnvalue _returnvalue_19 (Class|KismetMathLibrary|QuatRotator (Class|KismetMathLibrary|QuatSlerp (Math|Conversions|ToQuaternion(Rotator) (Transformation|GetActorRotation _returnvalue)) (Math|Conversions|ToQuaternion(Rotator) (Math|Rotator|FindLookatRotation _returnvalue_4 _returnvalue_5)) (* DeltaSeconds _turninterpspeed))))
              (goto _label_2)))
          (elif (== (Variables|ButterflyState|GetButterflyState) 3)
            (if _desiredvisible
              (Rendering|SetActorHiddenInGame _returnvalue false)
              (Variables|ButterflyState|SetButterflyState 0))
            (elif _desiredvisible
              (Transformation|SetActorLocationAndRotation _returnvalue (+ _returnvalue_6 (* (Math|Vector|GetForwardVector _returnvalue_30) _returnvalue_18)) _returnvalue_30)
              (if (<= _returnvalue_24 _arrivaltolerance)
                (Variables|Default|SetCurrentDistance _returnvalue_12)
                (Variables|ButterflyState|SetButterflyState 1))
              (else
                (goto _label_2)))))))
    (elif (<= (Math|Vector|VectorLength (- (Transformation|GetActorLocation _returnvalue) _returnvalue_5)) _arrivaltolerance)
      (goto _label_3)
      (else
        (goto _label)))))

(fn SetupSpline
  (params (InSplineComp :type Spline%20Component%20Object%20Reference))
  (bind _returnvalue (Components|GetOwner))
  (Variables|Default|SetSplineComp InSplineComp)
  (Transformation|SetActorLocationAndRotation _returnvalue (Spline|GetLocationatDistanceAlongSpline InSplineComp 0.0 "World") (Spline|GetRotationatDistanceAlongSpline InSplineComp 0.0 "World"))
  (Rendering|SetActorHiddenInGame _returnvalue true)
  (Variables|ButterflyState|SetButterflyState 3)
  (Variables|Default|SetCurrentDistance 0.0))

(fn SetDesiredVisibleState
  (params (bInDesiredVisible :type Boolean))
  (Variables|ButterflyState|SetDesiredVisible bInDesiredVisible))