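; Child butterfly Blueprint that follows a referenced spline path and shows or hides itself according to a global butterfly control value.
; On BeginPlay it caches the game instance and hands the PathRef spline to its BPSplineFollower component.
; BeginPlay and every Tick set the follower's desired visibility, true only while the game instance MAController's ButterflyControlValue exceeds this butterfly's SpawnThreshold plus a small margin.
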(event EventBeginPlay
  (bind _bp_splinefollower (Variables|Default|GetBP_SplineFollower))
  (bind _pathref (Variables|Default|GetPathRef))
  (|CallParentFunction)
  (bind _asbp_game_instance (Utilities|Casting|CastToBP_GameInstance (Game|GetGameInstance)))
  (Variables|/Game/Adohi_Dev/BPs/MAAssets/Butterflies/BP_SplineFollower.BP_SplineFollower_C|SetSplineParent _bp_splinefollower _pathref)
  (Utilities|FlowControl|Sequence
    (:then_0
      (Default|SetupSpline _bp_splinefollower (Actor|GetComponentbyClass _pathref "/Script/Engine.SplineComponent")))
    (:then_1
      (Default|SetDesiredVisibleState _bp_splinefollower (not (<= (Variables|/Game/Adohi_Dev/BPs/MAControls/BP_MAController.BP_MAController_C|GetButterflyControlValue (Variables|/Game/Adohi_Dev/CMS/Blueprints/BP_GameInstance.BP_GameInstance_C|GetMAController _asbp_game_instance)) (+ (Math|Conversions|ToFloat(Integer) (Variables|Default|GetSpawnThreshold)) 0.01)))))))

(event Collision|EventActorBeginOverlap
  (params (OtherActor :type Actor%20Object%20Reference))
  (|CallParentFunction OtherActor) ; FAI:auto_5f151532\nThis node is disabled and will not be called.\nDrag off pins to build functionality.
)

(event EventTick
  (params (DeltaSeconds :type Float%20%28single-precision%29))
  (|CallParentFunction DeltaSeconds)
  (Default|SetDesiredVisibleState (Variables|Default|GetBP_SplineFollower) (not (<= (Variables|/Game/Adohi_Dev/BPs/MAControls/BP_MAController.BP_MAController_C|GetButterflyControlValue (Variables|/Game/Adohi_Dev/CMS/Blueprints/BP_GameInstance.BP_GameInstance_C|GetMAController (stale EventBeginPlay _asbp_game_instance))) (+ (Math|Conversions|ToFloat(Integer) (Variables|Default|GetSpawnThreshold)) 0.01)))))

(fn ConstructionScript
  (|CallParentFunction))