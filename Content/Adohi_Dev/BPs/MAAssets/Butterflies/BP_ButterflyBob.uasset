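; Component that bobs its owner's static mesh up and down, apparently for butterflies.
; BeginPlay caches the mesh's relative location and can randomize phase so instances desync.
; Tick sets relative Z from a game-time sine, or in FlapPop mode kicks height on each upward zero crossing and decays it linearly.
; A wrapped cycle phase also accumulates, but the height calculation ignores it and adds a separate offset variable.
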(event EventBeginPlay
  (if (Utilities|IsValid (Variables|ButterflyBob|GetTargetMeshComponent))
    _
    (else
      (Variables|ButterflyBob|SetTargetMeshComponent (Actor|GetComponentbyClass (Components|GetOwner) "/Script/Engine.StaticMeshComponent"))))
  (if (Variables|ButterflyBob|GetbRandomizePhaseOnBeginPlay)
    (Variables|ButterflyBob|SetPhaseOffset (Math|Random|RandomFloatinRange 0.0 6.283185307179586)))
  (Variables|ButterflyBob|SetInitialRelativeLocation (.Location (Math|Transform|BreakTransform (Transformation|GetRelativeTransform (Variables|ButterflyBob|GetTargetMeshComponent)))))
  (Variables|ButterflyBob|SetFlapPop_LastSin 1.0)
  (Variables|ButterflyBob|SetFlapPop_CurrentZ 0.0))

(event EventTick
  (params (DeltaSeconds :type Float%20%28single-precision%29))
  (bind _returnvalue (Utilities|Time|GetGameTimeinSeconds))
  (bind _targetmeshcomponent (Variables|ButterflyBob|GetTargetMeshComponent))
  (bind _bobfrequency (Variables|ButterflyBob|GetBobFrequency))
  (bind _phaseoffset (Variables|ButterflyBob|GetPhaseOffset))
  (bind _bobamplitude (Variables|ButterflyBob|GetBobAmplitude))
  (bind _initialrelativelocation (Variables|ButterflyBob|GetInitialRelativeLocation))
  (bind _bflappopmode (Variables|ButterflyBob|GetbFlapPopMode))
  (bind (_x _y _z) (Math|Vector|BreakVector _initialrelativelocation))
  (bind _returnvalue_2 (* _returnvalue _bobfrequency))
  (bind _returnvalue_3 (+ _returnvalue_2 _phaseoffset))
  (bind _returnvalue_4 (Math|Trig|Sin(Radians) _returnvalue_3))
  (Utilities|FlowControl|Sequence
    (:then_0
      (if (>= (+ (Variables|ButterflyBob|GetBobCyclePhase) (* DeltaSeconds _bobfrequency)) 6.283185307179586)
        (Variables|ButterflyBob|SetBobCyclePhase (.Remainder (Math|Float|Division(WholeandRemainder) (+ (Variables|ButterflyBob|GetBobCyclePhase) (* DeltaSeconds _bobfrequency)) 6.283185307179586)))
        (else
          (Variables|ButterflyBob|SetBobCyclePhase (+ (Variables|ButterflyBob|GetBobCyclePhase) (* DeltaSeconds _bobfrequency))))))
    (:then_1
      (if (Utilities|IsValid _targetmeshcomponent)
        (if _bflappopmode
          (Variables|ButterflyBob|SetFlapPop_CurrentZ (+ (Math|Interpolation|FInterptoConstant (Variables|ButterflyBob|GetFlapPop_CurrentZ) 0.0 DeltaSeconds (* _bobfrequency (Variables|ButterflyBob|GetFlapPopDecayScale))) (Math|Float|SelectFloat _bobamplitude 0.0 (and (< (Variables|ButterflyBob|GetFlapPop_LastSin) 0.0) (>= _returnvalue_4 0.0)))))
          (Variables|ButterflyBob|SetFlapPop_LastSin _returnvalue_4))
        (Transformation|SetRelativeLocation _targetmeshcomponent (Math|Vector|MakeVector _x _y (+ (Math|Float|SelectFloat (+ _z (Variables|ButterflyBob|GetFlapPop_CurrentZ)) (+ _z (* _returnvalue_4 _bobamplitude)) _bflappopmode) (Variables|ButterflyBob|GetBobPerCycleHeightOffset))) false false)))))