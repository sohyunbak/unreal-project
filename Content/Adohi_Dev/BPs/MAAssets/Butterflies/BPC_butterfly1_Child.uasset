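; Child Blueprint of a butterfly actor that follows a spline path and shows only when a controller value is high enough.
; On BeginPlay it runs the parent logic and assigns PathRef as the spline for its BPSplineFollower.
; On BeginPlay and every Tick it hides itself unless MAController's ButterflyControlValue exceeds its SpawnThreshold plus a small margin, so visibility is toggled rather than the actor spawned.
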(event EventBeginPlay
  (|CallParentFunction)
  (Variables|/Game/Adohi_Dev/BPs/MAAssets/Butterflies/BP_SplineFollower.BP_SplineFollower_C|SetSplineParent (Variables|Default|GetBP_SplineFollower) (Variables|Default|GetPathRef))
  (Rendering|SetActorHiddenInGame (<= (Variables|/Game/Adohi_Dev/BPs/MAControls/BP_MAController.BP_MAController_C|GetButterflyControlValue (Variables|Default|GetMAController)) (+ (Variables|Default|GetSpawnThreshold) 0.01))))

(event Collision|EventActorBeginOverlap
  (params (OtherActor :type Actor%20Object%20Reference))
  (|CallParentFunction OtherActor) ; This node is disabled and will not be called.\nDrag off pins to build functionality.
)

(event EventTick
  (params (DeltaSeconds :type Float%20%28single-precision%29))
  (|CallParentFunction DeltaSeconds)
  (Rendering|SetActorHiddenInGame (<= (Variables|/Game/Adohi_Dev/BPs/MAControls/BP_MAController.BP_MAController_C|GetButterflyControlValue (Variables|Default|GetMAController)) (+ (Variables|Default|GetSpawnThreshold) 0.01))))

(fn ConstructionScript
  (|CallParentFunction))