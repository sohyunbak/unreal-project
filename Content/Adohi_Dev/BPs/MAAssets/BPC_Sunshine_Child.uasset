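; Sunshine child Blueprint that drives the glow of its static mesh from a shared control value.
; On BeginPlay it creates and stores a dynamic material instance from the mesh's first material slot.
; Every Tick, ApplyValue sets the Glow scalar parameter by lerping between MinValue and MaxValue, using MAController's RayControlVar as alpha.
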(event Custom|ApplyValue
  (bind _dynamicmaterial (Variables|Default|GetDynamicMaterial))
  (Utilities|IsValid _dynamicmaterial
    (:Is%20Valid
      (Rendering|Material|SetScalarParameterValue _dynamicmaterial "Glow" (Math|Float|Lerp (Variables|Default|GetMinValue) (Variables|Default|GetMaxValue) (Variables|/Game/Adohi_Dev/BPs/MAControls/BP_MAController.BP_MAController_C|GetRayControlVar (Variables|Default|GetMAController))) :!class /Script/Engine.MaterialInstanceDynamic))))

(event EventBeginPlay
  (bind _staticmesh (Variables|Default|GetStaticMesh))
  (|CallParentFunction)
  (bind _returnvalue (Rendering|Material|CreateDynamicMaterialInstance _staticmesh 0 (Rendering|Material|GetMaterial _staticmesh 0) "None" :!class /Script/Engine.PrimitiveComponent))
  (Variables|Default|SetDynamicMaterial _returnvalue))

(event Collision|EventActorBeginOverlap
  (params (OtherActor :type Actor%20Object%20Reference))
  (|CallParentFunction OtherActor) ; This node is disabled and will not be called.\nDrag off pins to build functionality.
)

(event EventTick
  (params (DeltaSeconds :type Float%20%28single-precision%29))
  (|CallParentFunction DeltaSeconds)
  (CallFunction|ApplyValue))

(fn ConstructionScript
  (|CallParentFunction))