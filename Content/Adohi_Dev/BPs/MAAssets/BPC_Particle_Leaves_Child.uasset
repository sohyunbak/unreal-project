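; Child particle Blueprint, named for leaves, whose particle system follows the MAController's FlowerParticleTrigger flag.
; BeginPlay runs the parent logic, then deactivates the particle system.
; Each Tick calls the parent, then passes the flag to SetEmitterEnable with an emitter name of None.
; An Activate/Deactivate branch on the same flag is left unconnected and never runs.
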(event EventBeginPlay
  (|CallParentFunction)
  (Components|Activation|Deactivate (Variables|Default|GetParticleSystem)))

(event Collision|EventActorBeginOverlap
  (params (OtherActor :type Actor%20Object%20Reference))
  (|CallParentFunction OtherActor) ; This node is disabled and will not be called.\nDrag off pins to build functionality.
)

(event EventTick
  (params (DeltaSeconds :type Float%20%28single-precision%29))
  (|CallParentFunction DeltaSeconds)
  (Effects|Components|ParticleSystem|SetEmitterEnable (Variables|Default|GetParticleSystem) "None" (Variables|/Game/Adohi_Dev/BPs/MAControls/BP_MAController.BP_MAController_C|GetFlowerParticleTrigger (Variables|Default|GetMAController))))

(fn ConstructionScript
  (|CallParentFunction))