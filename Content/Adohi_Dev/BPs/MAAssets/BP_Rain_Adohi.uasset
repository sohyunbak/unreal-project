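; BP_Rain_Adohi is an actor that drives a rain effect on a glass mesh through its material.
; On BeginPlay it creates a dynamic material instance from the Glass component's first material.
; Every tick it sets the material's ClampMax parameter by interpolating between MinValue and MaxValue, using the WindowControlVar value read from MAController.
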(event Custom|ApplyValue
  (Utilities|IsValid (Variables|Default|GetDynamicMat)
    (:Is%20Valid
      ;[0.15 0.15 0.15 0.5] APPLY MATERIAL VALUE
      (Rendering|Material|SetScalarParameterValue (Variables|Default|GetDynamicMat) "ClampMax" (Math|Float|Lerp (Variables|Default|GetMinValue) (Variables|Default|GetMaxValue) (Variables|/Game/Adohi_Dev/BPs/MAControls/BP_MAController.BP_MAController_C|GetWindowControlVar (Variables|Default|GetMAController))) :!class /Script/Engine.MaterialInstanceDynamic))))

(event EventBeginPlay
  (bind _glass (Variables|Default|GetGlass))
  ;[0.15 0.15 0.15 0.5] INIT / BeginPlay
  (bind _returnvalue (Rendering|Material|CreateDynamicMaterialInstance _glass 0 (Rendering|Material|GetMaterial _glass 0) "None" :!class /Script/Engine.PrimitiveComponent))
  (Variables|Default|SetDynamicMat _returnvalue))

(event Collision|EventActorBeginOverlap
  (params (OtherActor :type Actor%20Object%20Reference)))

(event EventTick
  (params (DeltaSeconds :type Float%20%28single-precision%29))
  (CallFunction|ApplyValue))

(fn ConstructionScript)