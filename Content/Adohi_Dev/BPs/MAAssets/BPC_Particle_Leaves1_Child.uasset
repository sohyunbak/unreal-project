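; Child Blueprint of a leaves particle actor that shows its effect only while the MA controller's flower particle trigger is set.
; BeginPlay deactivates the particle system.
; Tick then polls MAController.FlowerParticleTrigger every frame, activating or deactivating the system to match.
; Unconnected SetEmitterEnable nodes and a disabled overlap event do nothing.
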(event EventBeginPlay
  (|CallParentFunction)
  (Components|Activation|Deactivate (Variables|Default|GetParticleSystem)))

(event Collision|EventActorBeginOverlap
  (params (OtherActor :type Actor%20Object%20Reference))
  (|CallParentFunction OtherActor) ; This node is disabled and will not be called.\nDrag off pins to build functionality.
)

(event EventTick
  (params (DeltaSeconds :type Float%20%28single-precision%29))
  (bind _particlesystem (Variables|Default|GetParticleSystem))
  (|CallParentFunction DeltaSeconds)
  (if (Variables|/Game/Adohi_Dev/BPs/MAControls/BP_MAController.BP_MAController_C|GetFlowerParticleTrigger (Variables|Default|GetMAController))
    (Components|Activation|Activate _particlesystem false)
    (else
      (Components|Activation|Deactivate _particlesystem))))

(fn ConstructionScript
  (|CallParentFunction))