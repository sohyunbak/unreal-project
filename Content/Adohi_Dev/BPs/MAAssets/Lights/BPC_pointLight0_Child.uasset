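; BPC_pointLight0_Child is a child Blueprint of a point light whose brightness is driven by a shared control variable.
; On BeginPlay it casts and caches the BP_GameInstance.
; Every Tick it sets the light intensity by interpolating between the game instance's Light0 minimum and maximum values, using the MAController's RayControlVar as alpha.
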(event EventBeginPlay
  (|CallParentFunction)
  (bind _asbp_game_instance (Utilities|Casting|CastToBP_GameInstance (Game|GetGameInstance))))

(event Collision|EventActorBeginOverlap
  (params (OtherActor :type Actor%20Object%20Reference))
  (|CallParentFunction OtherActor) ; This node is disabled and will not be called.\nDrag off pins to build functionality.
)

(event EventTick
  (params (DeltaSeconds :type Float%20%28single-precision%29))
  (|CallParentFunction DeltaSeconds)
  (Rendering|Components|Light|SetIntensity (Variables|Default|GetPointLight) (Math|Float|Lerp (Variables|/Game/Adohi_Dev/CMS/Blueprints/BP_GameInstance.BP_GameInstance_C|GetLight0MinValue (stale EventBeginPlay _asbp_game_instance)) (Variables|/Game/Adohi_Dev/CMS/Blueprints/BP_GameInstance.BP_GameInstance_C|GetLight0MaxValue (stale EventBeginPlay _asbp_game_instance)) (Variables|/Game/Adohi_Dev/BPs/MAControls/BP_MAController.BP_MAController_C|GetRayControlVar (Variables|/Game/Adohi_Dev/CMS/Blueprints/BP_GameInstance.BP_GameInstance_C|GetMAController (stale EventBeginPlay _asbp_game_instance))))))

(fn ConstructionScript
  (|CallParentFunction))