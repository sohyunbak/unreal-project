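; BP_DummyDataGenerator produces a continuously changing integer test value between MinValue and MaxValue, standing in for live data.
; On BeginPlay it gets BP_GameInstance and starts a looping timer that recomputes CurrentValue every TimerTick.
; Each update samples 1D Perlin noise over game time at the game instance's noise speed, stretches it with an edge contrast factor, clamps it, and lerps it into the range.
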(event Custom|SetValue
  (Variables|Default|SetCurrentValue (Math|Float|Round (Math|Float|Lerp (Math|Conversions|ToFloat(Integer) (Variables|Default|GetMinValue)) (Math|Conversions|ToFloat(Integer) (Variables|Default|GetMaxValue)) (Math|Float|Clamp(Float) (+ (* (- (Math|Float|MapRangeClamped (Class|KismetMathLibrary|PerlinNoise1D (* (Utilities|Time|GetGameTimeinSeconds) (Variables|/Game/Adohi_Dev/CMS/Blueprints/BP_GameInstance.BP_GameInstance_C|GetDummyDataNoiseSpeed (stale EventBeginPlay _asbp_game_instance)))) -1.0 1.0 0.0 1.0) 0.5) (Variables|Default|GetNoiseEdgeContrast)) 0.5) 0.0 1.0)))))

(event EventBeginPlay
  (bind _asbp_game_instance (Utilities|Casting|CastToBP_GameInstance (Game|GetGameInstance)))
  (Utilities|Time|SetTimerbyEvent (delegate Custom|SetValue) (Variables|Default|GetTimerTick) true))

(fn ConstructionScript)