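; Controller that turns a people count, from VisionRelay or a dummy DataGenerator, into phase-based control values for window, ray and flower particle effects.
; Each tick interpolates and normalizes the count, with an optional manual value replacing the normalized result.
; The smoothed count selects a phase from PhaseConfig thresholds, which drives those effect values.
; Debug keys toggle source and manual mode or nudge the value, and a looping timer logs the count.
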(event Custom|DataLogger
  (bind _visionrelay (Variables|Default|GetVisionRelay))
  (bind _minpeoplecount (Variables|Default|GetMinPeopleCount))
  (bind _maxpeoplecount (Variables|Default|GetMaxPeopleCount))
  (bind _datagenerator (Variables|Default|GetDataGenerator))
  (bind _usevisionrelay (Variables|Default|GetUseVisionRelay))
  (bind _currentpeoplecount (Variables|/Game/CMS/Blueprints/BP_VisionRelayDataReceiver.BP_VisionRelayDataReceiver_C|GetCurrentPeopleCount _visionrelay))
  (bind _currentvalue (Variables|/Game/Adohi_Dev/BPs/MAControls/BP_DummyDataGenerator.BP_DummyDataGenerator_C|GetCurrentValue _datagenerator))
  (if _usevisionrelay
    (Development|PrintString (Utilities|String|Append "VisionRelay PeopleCount:" (Utilities|String|ToString(Integer) _currentpeoplecount)))
    (else
      (Development|PrintString (Utilities|String|Append "DummyData PeopleCount:" (Utilities|String|ToString(Integer) _currentvalue)))))
  (bind _interpolatedpeoplecount (CallFunction|InterpolateData (Math|Float|Truncate (Math|Float|SelectFloat (Math|Conversions|ToFloat(Integer) _currentpeoplecount) (Math|Conversions|ToFloat(Integer) _currentvalue) _usevisionrelay)) (Variables|Default|GetInterpolatedPeopleCount) 1.0 _minpeoplecount _maxpeoplecount))
  (Variables|Default|SetInterpolatedPeopleCount _interpolatedpeoplecount)
  (Variables|Default|SetNormalizedData (Math|Float|SelectFloat (Variables|Default|GetCustomData) (Math|Float|NormalizetoRange _interpolatedpeoplecount (Math|Conversions|ToFloat(Integer) _minpeoplecount) (Math|Conversions|ToFloat(Integer) _maxpeoplecount)) (Variables|Default|GetUseCustomValue))))

(event EventTick
  (params (DeltaSeconds :type Float%20%28single-precision%29))
  (bind _phaseconfig (Variables|Default|GetPhaseConfig))
  (bind _minpeoplecount (Variables|Default|GetMinPeopleCount))
  (bind _maxpeoplecount (Variables|Default|GetMaxPeopleCount))
  (Utilities|FlowControl|Sequence
    (:then_0
      (Utilities|FlowControl|Sequence
        (:then_0
          (bind _interpolatedpeoplecount (CallFunction|InterpolateData (Math|Float|Truncate (Math|Float|SelectFloat (Math|Conversions|ToFloat(Integer) (Variables|/Game/CMS/Blueprints/BP_VisionRelayDataReceiver.BP_VisionRelayDataReceiver_C|GetCurrentPeopleCount (Variables|Default|GetVisionRelay))) (Math|Conversions|ToFloat(Integer) (Variables|/Game/Adohi_Dev/BPs/MAControls/BP_DummyDataGenerator.BP_DummyDataGenerator_C|GetCurrentValue (Variables|Default|GetDataGenerator))) (Variables|Default|GetUseVisionRelay))) (Variables|Default|GetInterpolatedPeopleCount) 1.0 _minpeoplecount _maxpeoplecount))
          (Variables|Default|SetInterpolatedPeopleCount _interpolatedpeoplecount)
          (Variables|Default|SetNormalizedData (Math|Float|SelectFloat (Variables|Default|GetCustomData) (Math|Float|NormalizetoRange _interpolatedpeoplecount (Math|Conversions|ToFloat(Integer) _minpeoplecount) (Math|Conversions|ToFloat(Integer) _maxpeoplecount)) (Variables|Default|GetUseCustomValue))))
        (:then_1
          (Utilities|FlowControl|Gate true
            (:Exit
              (Variables|Default|SetCustomData (Math|Float|Clamp(Float) (+ (Variables|Default|GetCustomData) -0.01))))))
        (:then_2
          (Utilities|FlowControl|Gate true
            (:Exit
              (Variables|Default|SetCustomData (Math|Float|Clamp(Float) (+ (Variables|Default|GetCustomData) 0.01))))))))
    (:then_1
      (bind _array_element (Utilities|Array|ForEachLoopwithBreak (Variables|Default|GetPhaseConfig) :!label _label)
        (:LoopBody
          (if (< (Variables|Default|GetInterpolatedPeopleCount) (.Threshold (Utilities|Struct|BreakS_PhaseConfig _array_element)))
            (Variables|Default|SetCurrentPhase (.Phase (Utilities|Struct|BreakS_PhaseConfig _array_element)))
            (goto _label Break)))))
    (:then_2
      (Variables|Default|SetFlowerParticleTrigger (Utilities|Enum|Equal(Enum) (Variables|Default|GetCurrentPhase) "NewEnumerator3") :!label _label_2)
      (switch Utilities|FlowControl|Switch|SwitchonE_MAPhase (Variables|Default|GetCurrentPhase)
        (:NewEnumerator0
          (Variables|Default|SetWindowControlVar (Math|Interpolation|FInterpTo (Variables|Default|GetWindowControlVar) 0.0 (Utilities|Time|GetWorldDeltaSeconds) (Variables|Default|GetWindowControlLerpSpeed))))
        (:NewEnumerator1
          (Variables|Default|SetWindowControlVar (Math|Interpolation|FInterpTo (Variables|Default|GetWindowControlVar) 1.0 (Utilities|Time|GetWorldDeltaSeconds) (Variables|Default|GetWindowControlLerpSpeed))))
        (:NewEnumerator2
          (Variables|Default|SetRayControlVar (Math|Float|MapRangeClamped (Variables|Default|GetInterpolatedPeopleCount) (.Threshold (Utilities|Struct|BreakS_PhaseConfig (Utilities|Array|Get(acopy) _phaseconfig 1))) (.Threshold (Utilities|Struct|BreakS_PhaseConfig (Utilities|Array|Get(acopy) _phaseconfig 2))) 0.0 1.0)))
        (:NewEnumerator3
          (goto _label_2))))))

(event Collision|EventActorBeginOverlap
  (params (OtherActor :type Actor%20Object%20Reference)))

(event EventBeginPlay
  (Utilities|Time|SetTimerbyEvent (delegate Custom|DataLogger) 1.0 true))

(event Input|KeyboardEvents|SpaceBar
  (params (Key :type Key%20Structure :default "None"))
  (:Pressed
    (Variables|Default|SetUseVisionRelay (not (Variables|Default|GetUseVisionRelay)))))

(event Input|KeyboardEvents|X
  (params (Key :type Key%20Structure :default "None"))
  (:Pressed
    (Variables|Default|SetUseCustomValue (not (Variables|Default|GetUseCustomValue)))
    (if (Variables|Default|GetUseCustomValue)
      (Development|PrintString "Custom Value Mode: On")
      (else
        (Development|PrintString "Custom Value Mode: Off")))))

(event Input|KeyboardEvents|Left
  (params (Key :type Key%20Structure :default "None"))
  (:Pressed
    (Utilities|FlowControl|Gate true) ; enters at Open
  )
  (:Released
    (Utilities|FlowControl|Gate true) ; enters at Close
  ))

(event Input|KeyboardEvents|Right
  (params (Key :type Key%20Structure :default "None"))
  (:Pressed
    (Utilities|FlowControl|Gate true) ; enters at Open
  )
  (:Released
    (Utilities|FlowControl|Gate true) ; enters at Close
  ))

(fn ConstructionScript)

(fn OnRepCurrentPhase
  (switch Utilities|FlowControl|Switch|SwitchonE_MAPhase (Variables|Default|GetCurrentPhase)))