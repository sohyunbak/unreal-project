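; BP_Rain is an actor that eases the Normal_Intensity parameter of a frosted glass material, apparently for a rain effect on a window.
; Each tick, threshold mode picks the start or end value from InputValue, FInterpTo smooths toward it, and ApplyValue writes it if DynamicMat is valid.
; BeginPlay creates the dynamic instance on Glass but sets DynamicMat to None, so the write is skipped as wired.
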(event Custom|ApplyValue
  ;[0.15 0.15 0.15 0.5] APPLY MATERIAL VALUE
  (Utilities|IsValid (Variables|Default|GetDynamicMat)
    (:Is%20Valid
      (Rendering|Material|SetScalarParameterValue (Variables|Default|GetDynamicMat) "Normal_Intensity" (Variables|Default|GetCurrentValue) :!class /Script/Engine.MaterialInstanceDynamic))))

(event Custom|UpdateTarget
  ;[0.15 0.15 0.15 0.5] TARGET VALUE LOGIC
  (if (Variables|Default|GetUseThresholdMode)
    (if (>= (Variables|Default|GetInputValue) (Variables|Default|GetThresholdValue))
      (Variables|Default|SetTargetValue (Variables|Default|GetEndValue))
      (else
        (Variables|Default|SetTargetValue (Variables|Default|GetStartValue))))))

(event EventBeginPlay
  ;[0.15 0.15 0.15 0.5] INIT / BeginPlay
  (Rendering|Material|CreateDynamicMaterialInstance (Variables|Default|GetGlass) 0 "/Game/GlassMirrorsWindows/Materials/MIC_Glass_Frosted_Noise.MIC_Glass_Frosted_Noise" "None" :!class /Script/Engine.PrimitiveComponent)
  (Variables|Default|SetDynamicMat 0)
  (Variables|Default|SetCurrentValue (Variables|Default|GetStartValue))
  (CallFunction|ApplyValue))

(event Collision|EventActorBeginOverlap
  (params (OtherActor :type Actor%20Object%20Reference)))

(event EventTick
  (params (DeltaSeconds :type Float%20%28single-precision%29))
  ;[0.15 0.15 0.15 0.5] TICK / SMOOTH INTERPOLATION
  (CallFunction|UpdateTarget)
  (Variables|Default|SetCurrentValue (Math|Interpolation|FInterpTo (Variables|Default|GetCurrentValue) (Variables|Default|GetTargetValue) DeltaSeconds (Variables|Default|GetInterpSpeed)))
  (CallFunction|ApplyValue))

(fn ConstructionScript)