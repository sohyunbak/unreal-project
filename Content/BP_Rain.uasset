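; BP_Rain is an actor meant to animate the Normal_Intensity of a frosted glass material, presumably for a rain effect.
; Each Tick picks StartValue or EndValue by comparing InputValue to a threshold when threshold mode is on, then eases CurrentValue toward it with FInterpTo.
; The result goes to DynamicMat if valid, but the material setup is disconnected from BeginPlay and nothing here assigns that variable or InputValue.
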(event Custom|ApplyValue
  (Utilities|IsValid (Variables|Default|GetDynamicMat)
    (:Is%20Valid
      (Rendering|Material|SetScalarParameterValue (Variables|Default|GetDynamicMat) "Normal_Intensity" (Variables|Default|GetCurrentValue) :!class /Script/Engine.MaterialInstanceDynamic))))

(event Custom|UpdateTarget
  ;[0.15 0.15 0.15 0.5] FAI:auto_4afebef4
  ; INIT / BeginPlay
  (if (Variables|Default|GetUseThresholdMode)
    (if (>= (Variables|Default|GetInputValue) (Variables|Default|GetThresholdValue))
      ;[0.15 0.15 0.15 0.5] FAI:auto_5320d4d3
      ; TARGET VALUE LOGIC
      (Variables|Default|SetTargetValue (Variables|Default|GetEndValue))
      (else
        (Variables|Default|SetTargetValue (Variables|Default|GetStartValue))))))

(event EventBeginPlay)

(event Collision|EventActorBeginOverlap
  (params (OtherActor :type Actor%20Object%20Reference)))

(event EventTick
  (params (DeltaSeconds :type Float%20%28single-precision%29))
  (CallFunction|UpdateTarget)
  (Variables|Default|SetCurrentValue (Math|Interpolation|FInterpTo (Variables|Default|GetCurrentValue) (Variables|Default|GetTargetValue) DeltaSeconds (Variables|Default|GetInterpSpeed)))
  (CallFunction|ApplyValue))

(fn ConstructionScript)